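; Fire projectile actor ("Огонь") that flies toward the point under the mouse cursor and damages NPS actors it hits.
; On BeginPlay it reads the cursor trace and uses MoveComponentTo over four seconds, feeding world X/Y with zero Z as a relative target.
; Sphere1 hits spawn an explosion at the impact point.
; Only an NPS hit subtracts 100 HP and destroys the projectile.
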(event OnComponentHit(Sphere1)
  (params (HitComponent :type Primitive%20Component%20Object%20Reference) (OtherActor :type Actor%20Object%20Reference) (OtherComp :type Primitive%20Component%20Object%20Reference) (NormalImpulse :type Vector :default "0, 0, 0") (Hit :type Hit%20Result%20Structure%20%28by%20ref%29))
  (bind (_bblockinghit _binitialoverlap _time _distance _location _impactpoint _normal _impactnormal _physmat _hitactor) (Collision|BreakHitResult Hit))
  (Effects|SpawnEmitteratLocation "/Game/FXVarietyPack/Particles/P_ky_explosion.P_ky_explosion" _impactpoint)
  (bind _asnps (Utilities|Casting|CastToNPS _hitactor))
  (bind _output_get (Variables|/Game/Blueprints/NPS.NPS_C|SetHP _asnps (- (stale _output_get) 100)))
  (Actor|DestroyActor))

(event EventBeginPlay
  (bind _returnvalue (Game|GetPlayerController 0))
  (bind _hitresult (Game|Player|GetHitResultUnderCursorbyChannel _returnvalue "TraceTypeQuery1" true))
  (bind _location (Collision|BreakHitResult _hitresult))
  (bind (_x _y) (Math|Vector|BreakVector _location))
  (Components|MoveComponentTo 0 (Math|Vector|MakeVector _x _y 0.0) "0, 0, 0" false false 4.0 false))

(fn ConstructionScript)