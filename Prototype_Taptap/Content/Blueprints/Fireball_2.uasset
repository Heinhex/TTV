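; Fireball actor that reacts to its sphere component hitting something and destroys itself three seconds later.
; A hit on an NPS opens a gate fed by Tick, but the gate drives nothing.
; Nodes for moving toward the point under the cursor and for subtracting NPS health with a debug print are disconnected, so the file applies no movement or damage.
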(event OnComponentHit(Sphere1)
  (params (HitComponent :type Primitive%20Component%20Object%20Reference) (OtherActor :type Actor%20Object%20Reference) (OtherComp :type Primitive%20Component%20Object%20Reference) (NormalImpulse :type Vector :default "0, 0, 0") (Hit :type Hit%20Result%20Structure%20%28by%20ref%29))
  (Utilities|FlowControl|Sequence
    (:then_0
      (bind _asnps (Utilities|Casting|CastToNPS OtherActor))
      (Utilities|FlowControl|Gate true) ; enters at Open
    )
    (:then_1
      (Utilities|FlowControl|Delay 3.0)
      (Actor|DestroyActor)
      (Utilities|FlowControl|Gate true) ; enters at Close
    )))

(event EventBeginPlay)

(event Collision|EventActorBeginOverlap
  (params (OtherActor :type Actor%20Object%20Reference)))

(event EventTick
  (params (DeltaSeconds :type Float%20%28single-precision%29))
  (Utilities|FlowControl|Gate true))

(fn ConstructionScript)