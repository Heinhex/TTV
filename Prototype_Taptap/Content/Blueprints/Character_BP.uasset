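; Player character with axis movement, a configurable spring-arm camera meant to stay locked on X, and death and respawn handling.
; R or Dead hides the player and starts the HUD death timer; Alive! teleports to a fixed spawn and restores health.
; Keys 1–3 refresh HUD cards and spend mana, with key 1 also spawning a fireball.
; Tick forwards to an empty StepaEVENTS hook; bush overlap only resets grass material on exit, as the highlight is unwired.
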(event OnComponentBeginOverlap(Sphere1)
  (params (OverlappedComponent :type Primitive%20Component%20Object%20Reference) (OtherActor :type Actor%20Object%20Reference) (OtherComp :type Primitive%20Component%20Object%20Reference) (OtherBodyIndex :type Integer) (bFromSweep :type Boolean) (SweepResult :type Hit%20Result%20Structure%20%28by%20ref%29))
  ;[1 1 1] Видимость кусов вокруг игрока.
  (bind _askust (Utilities|Casting|CastToKust OtherActor)))

(event OnComponentEndOverlap(Sphere1)
  (params (OverlappedComponent :type Primitive%20Component%20Object%20Reference) (OtherActor :type Actor%20Object%20Reference) (OtherComp :type Primitive%20Component%20Object%20Reference) (OtherBodyIndex :type Integer))
  ;[1 1 1] Видимость кусов вокруг игрока.
  (bind _askust (Utilities|Casting|CastToKust OtherActor))
  (Rendering|Material|SetMaterial (Variables|/Game/Blueprints/Kust.Kust_C|GetТрава _askust) 0 "/Game/Materials/Grass.Grass"))

(event Custom|Stepa%20EVENTS
  ;[1 1 1] Это вместо Event Tick, весь код делай тут
  (Utilities|FlowControl|Sequence))

(event Custom|Dead
  ;[1 1 1] Смерть игрока
  (Rendering|SetActorHiddenInGame true)
  (Collision|SetActorEnableCollision false)
  (bind _foundwidgets (Widget|GetAllWidgetsOfClass "/Game/Blueprints/NewWidgetBlueprint.NewWidgetBlueprint_C" true))
  (Default|Dead-timer (Utilities|Array|Get(acopy) _foundwidgets)))

(event Custom|Alive!
  ;[1 1 1] Воскрешение
  ;;[1 1 1] точка спавна, 1/3 точек спавна команды
  (Transformation|SetActorLocation (Math|Vector|MakeVector 2.92e+03 6.41e+03 1885.0) false false)
  (Rendering|SetActorHiddenInGame false)
  (Collision|SetActorEnableCollision true)
  (bind _asdannie (Utilities|Casting|CastToDannie (UserInterface|GetUserWidgetObject (Variables|Default|GetWidget))))
  (Variables|/Game/Blueprints/Dannie.Dannie_C|SetHP-now _asdannie 2e+02))

(event Custom|FB-1)

(event EventBeginPlay)

(event EventTick
  (params (DeltaSeconds :type Float%20%28single-precision%29))
  (bind _camera (Variables|Default|GetCamera))
  ;[0.06914 0 1] Это не трогай! Логику Event Tick пиши в Stepa EVENT
  ;;[1 1 1] Фиксация камеры на позиции. X - неподвижно
  (Transformation|SetWorldLocation _camera (Utilities|LockPosition _camera 3.5e+03) false false)
  ;;[1 1 1] TEST
  (CallFunction|StepaEVENTS))

(event Input|AxisEvents|InputAxisMoveForward
  (params (AxisValue :type Float%20%28single-precision%29))
  ;[1 1 1] Input
  (Pawn|Input|AddMovementInput (Transformation|GetActorForwardVector) AxisValue false))

(event Input|AxisEvents|InputAxisMoveRight
  (params (AxisValue :type Float%20%28single-precision%29))
  ;[1 1 1] Input
  (Pawn|Input|AddMovementInput (Transformation|GetActorRightVector) AxisValue false))

(event Input|KeyboardEvents|R
  (params (Key :type Key%20Structure :default "None"))
  (:Pressed
    ;[1 1 1] Смерть игрока
    (Rendering|SetActorHiddenInGame true)
    (Collision|SetActorEnableCollision false)
    (bind _foundwidgets (Widget|GetAllWidgetsOfClass "/Game/Blueprints/NewWidgetBlueprint.NewWidgetBlueprint_C" true))
    (Default|Dead-timer (Utilities|Array|Get(acopy) _foundwidgets))))

(event Input|KeyboardEvents|1
  (params (Key :type Key%20Structure :default "None"))
  (bind _mesh (Variables|Character|GetMesh))
  (bind _returnvalue (Transformation|GetWorldLocation _mesh))
  (bind (_x _y _z) (Math|Vector|BreakVector _returnvalue))
  (:Pressed
    (bind _foundwidgets (Widget|GetAllWidgetsOfClass "/Game/Blueprints/NewWidgetBlueprint.NewWidgetBlueprint_C" true))
    (Default|Respawn (Variables|/Game/Blueprints/NewWidgetBlueprint.NewWidgetBlueprint_C|GetKarta (Utilities|Array|Get(acopy) _foundwidgets)))
    (Variables|/Game/Blueprints/Karta.Karta_C|SetNewVar_0 (Variables|/Game/Blueprints/NewWidgetBlueprint.NewWidgetBlueprint_C|GetKarta (Utilities|Array|Get(acopy) _foundwidgets)) 5)
    (bind _output_get (Variables|/Game/Blueprints/NewWidgetBlueprint.NewWidgetBlueprint_C|SetMana-Now (Utilities|Array|Get(acopy) _foundwidgets) (- (stale _output_get) 2.0)))
    (Rendering|SetVisibility (Variables|Default|GetP_ky_fireBall) true false)
    (Game|SpawnActorfromClass "/Game/Blueprints/Fireball.Fireball_C" (Math|Transform|MakeTransform (Math|Vector|MakeVector _x (- _y -1.5e+02) _z)) "AlwaysSpawn" 0 0)
    (Variables|Default|SetOgon true)))

(event Input|KeyboardEvents|2
  (params (Key :type Key%20Structure :default "None"))
  (:Pressed
    (bind _foundwidgets (Widget|GetAllWidgetsOfClass "/Game/Blueprints/NewWidgetBlueprint.NewWidgetBlueprint_C" true))
    (Default|Respawn (Variables|/Game/Blueprints/NewWidgetBlueprint.NewWidgetBlueprint_C|GetKarta_1 (Utilities|Array|Get(acopy) _foundwidgets)))
    (Variables|/Game/Blueprints/Karta.Karta_C|SetNewVar_0 (Variables|/Game/Blueprints/NewWidgetBlueprint.NewWidgetBlueprint_C|GetKarta_1 (Utilities|Array|Get(acopy) _foundwidgets)) 6)
    (bind _output_get (Variables|/Game/Blueprints/NewWidgetBlueprint.NewWidgetBlueprint_C|SetMana-Now (Utilities|Array|Get(acopy) _foundwidgets) (- (stale _output_get) 5.0)))
    (Default|CustomEvent0 (Utilities|Array|Get(acopy) _foundwidgets))))

(event Input|KeyboardEvents|3
  (params (Key :type Key%20Structure :default "None"))
  (:Pressed
    (bind _foundwidgets (Widget|GetAllWidgetsOfClass "/Game/Blueprints/NewWidgetBlueprint.NewWidgetBlueprint_C" true))
    (Default|Respawn (Variables|/Game/Blueprints/NewWidgetBlueprint.NewWidgetBlueprint_C|GetKarta_2 (Utilities|Array|Get(acopy) _foundwidgets)))
    (Variables|/Game/Blueprints/Karta.Karta_C|SetNewVar_0 (Variables|/Game/Blueprints/NewWidgetBlueprint.NewWidgetBlueprint_C|GetKarta_2 (Utilities|Array|Get(acopy) _foundwidgets)) 7)
    (bind _output_get (Variables|/Game/Blueprints/NewWidgetBlueprint.NewWidgetBlueprint_C|SetMana-Now (Utilities|Array|Get(acopy) _foundwidgets) (- (stale _output_get) 1.0)))))

(fn ConstructionScript
  (bind _springarm (Variables|Default|GetSpringArm))
  (Variables|/Script/Engine.SpringArmComponent|SetSocketOffset _springarm (Math|Vector|MakeVector 0.0 0.0 (Variables|Default|GetCameraHigh)))
  (Variables|/Script/Engine.SpringArmComponent|SetTargetArmLength _springarm (Variables|Default|GetCameraDistance))
  (Transformation|SetRelativeRotation (Variables|Default|GetCamera) (Math|Rotator|MakeRotator 0.0 (Variables|Default|GetAngle) 0.0) false false))