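; NPS is a damageable actor that shows its name and health on a Dannie widget and takes hits from Fireball_2.
; BeginPlay and every Tick push the name and HP into the widget, and Tick destroys the actor once HP reaches zero or below.
; Overlaps on All_Firestar with Fireball_2 pass through a gate, reopened every Tick, to subtract a fixed amount of HP.
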(event OnComponentBeginOverlap(All_Firestar)
  (params (OverlappedComponent :type Primitive%20Component%20Object%20Reference) (OtherActor :type Actor%20Object%20Reference) (OtherComp :type Primitive%20Component%20Object%20Reference) (OtherBodyIndex :type Integer) (bFromSweep :type Boolean) (SweepResult :type Hit%20Result%20Structure%20%28by%20ref%29))
  (Utilities|Casting|CastToFireball_2 OtherActor)
  (Utilities|FlowControl|Gate true
    (:Exit
      (bind _output_get (Variables|Default|SetHP (- (stale _output_get) 50))))))

(event OnComponentEndOverlap(All_Firestar)
  (params (OverlappedComponent :type Primitive%20Component%20Object%20Reference) (OtherActor :type Actor%20Object%20Reference) (OtherComp :type Primitive%20Component%20Object%20Reference) (OtherBodyIndex :type Integer)))

(event EventBeginPlay
  (bind _asdannie (Utilities|Casting|CastToDannie (UserInterface|GetUserWidgetObject (Variables|Default|GetWidget))))
  (Variables|/Game/Blueprints/Dannie.Dannie_C|SetNamrd _asdannie (Variables|Default|GetNewVar_0))
  (Variables|/Game/Blueprints/Dannie.Dannie_C|SetHP-now _asdannie (Math|Conversions|ToFloat(Integer) (Variables|Default|GetHP))))

(event EventTick
  (params (DeltaSeconds :type Float%20%28single-precision%29))
  (Utilities|FlowControl|Sequence
    (:then_0
      (bind _asdannie (Utilities|Casting|CastToDannie (UserInterface|GetUserWidgetObject (Variables|Default|GetWidget))))
      (Variables|/Game/Blueprints/Dannie.Dannie_C|SetNamrd _asdannie (Variables|Default|GetNewVar_0))
      (Variables|/Game/Blueprints/Dannie.Dannie_C|SetHP-now _asdannie (Math|Conversions|ToFloat(Integer) (Variables|Default|GetHP))))
    (:then_1
      (if (<= (Variables|Default|GetHP) 0)
        (Actor|DestroyActor)))
    (:then_2
      (Utilities|FlowControl|Gate true) ; enters at Open
    )))

(fn ConstructionScript)